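; SpawnArea is an actor that spawns Enemy_BP enemies at random points within a box volume.
; On BeginPlay it sets the Start timeline's play rate from PlayRate, waits for Delaytime, then plays the timeline.
; The timeline's Dead event triggers each spawn, placing the enemy randomly within the Box extent centered on the root component's world location.
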(event `self.ReceiveBeginPlay`
  (`TimelineComponent.SetPlayRate` (`self.Start`) (`self.PlayRate`))
  (`KismetSystemLibrary.Delay` (`self.Delaytime`))
  (`Timeline|Start`
    (:`Dead`
      (`|SpawnActorFromClass` "/Game/Blueprints/Enemy_BP.Enemy_BP_C" (`KismetMathLibrary.MakeTransform` (`KismetMathLibrary.RandomPointInBoundingBox` (`SceneComponent.K2_GetComponentLocation` (`self.DefaultSceneRoot`)) (`BoxComponent.BoxExtent` (`self.Box`)))) "Undefined" "OverrideRootScale" null null))))

(fn `UserConstructionScript`)