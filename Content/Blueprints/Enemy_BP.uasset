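; Enemy_BP is an enemy actor that homes in on the player's MainStation_BP pawn and opens LevelBase when it overlaps it.
; On BeginPlay, the Moving0 timeline lerps the enemy from its current location toward the station's current location on every update, without sweep.
; A Death event destroys the actor; Tick and the construction script are empty.
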(event `self.ReceiveActorBeginOverlap`
  (params (OtherActor :type "Actor Object Reference"))
  (bind _asmain_station_bp (cast `/Game/Blueprints/MainStation_BP` OtherActor))
  (if (`self.IsOverlappingActor` _asmain_station_bp)
    (`GameplayStatics.OpenLevel` "LevelBase")))

(event `self.ReceiveBeginPlay`
  (bind _asmain_station_bp (cast `/Game/Blueprints/MainStation_BP` (`GameplayStatics.GetPlayerPawn` 0)))
  (bind (_direction _rimeformove) (`Timeline|Moving 0`)
    (:`Update`
      (`self.K2_SetActorLocation` (`KismetMathLibrary.VLerp` (`self.K2_GetActorLocation`) (`self.K2_GetActorLocation` _asmain_station_bp) _rimeformove)))))

(event `/Game/Blueprints/Deathable.Death`
  (`self.K2_DestroyActor`))

(fn `UserConstructionScript`)