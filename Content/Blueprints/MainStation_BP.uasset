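; MainStation_BP is a station actor that the player rotates and fits with turrets.
; Holding A or D sets flags that Tick reads to yaw the Box component by a fixed, frame-rate-dependent step, with A taking priority.
; Releasing a touch on one of four Block components sets the matching slot's Child Actor class to Turet1_BP.
; Touch events on the actor and on Box1 only print debug strings.
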(event `Key|A`
  (params (Key :type "Key Structure"))
  (:`Pressed`
    (set `self.A pressed` true))
  (:`Released`
    (set `self.A pressed` false)))

(event `self.ReceiveTick`
  (params (DeltaSeconds :type "Float (single-precision)"))
  (bind _box (`self.Box`))
  (if (`self.A pressed`)
    (`SceneComponent.K2_AddRelativeRotation` _box (struct :`Yaw` 0.5) false false)
    (elif (`self.D pressed`)
      (`SceneComponent.K2_AddRelativeRotation` _box (struct :`Yaw` -0.5) false false))))

(event `Key|D`
  (params (Key :type "Key Structure"))
  (:`Pressed`
    (set `self.D pressed` true))
  (:`Released`
    (set `self.D pressed` false)))

(event `self.ReceiveActorOnInputTouchBegin`
  (params (FingerIndex :type "ETouchIndex Enum" :default "Touch1"))
  (`KismetSystemLibrary.PrintString` "Hello"))

(event `self.Block1.OnInputTouchEnd`
  (params (FingerIndex :type "ETouchIndex Enum" :default "Touch1") (TouchedComponent :type "PrimitiveComponent Object Reference"))
  (`ChildActorComponent.SetChildActorClass` (`self.slot1Turet`) "/Game/Blueprints/Turet1_BP.Turet1_BP_C"))

(event `self.Block2.OnInputTouchEnd`
  (params (FingerIndex :type "ETouchIndex Enum" :default "Touch1") (TouchedComponent :type "PrimitiveComponent Object Reference"))
  (`ChildActorComponent.SetChildActorClass` (`self.slot2Turet`) "/Game/Blueprints/Turet1_BP.Turet1_BP_C"))

(event `self.Block3.OnInputTouchEnd`
  (params (FingerIndex :type "ETouchIndex Enum" :default "Touch1") (TouchedComponent :type "PrimitiveComponent Object Reference"))
  (`ChildActorComponent.SetChildActorClass` (`self.slot3turet`) "/Game/Blueprints/Turet1_BP.Turet1_BP_C"))

(event `self.Block4.OnInputTouchEnd`
  (params (FingerIndex :type "ETouchIndex Enum" :default "Touch1") (TouchedComponent :type "PrimitiveComponent Object Reference"))
  (`ChildActorComponent.SetChildActorClass` (`self.slot4turet`) "/Game/Blueprints/Turet1_BP.Turet1_BP_C"))

(event `self.Box1.OnInputTouchEnd`
  (params (FingerIndex :type "ETouchIndex Enum" :default "Touch1") (TouchedComponent :type "PrimitiveComponent Object Reference"))
  (`KismetSystemLibrary.PrintString` "smtrhing"))

(fn `UserConstructionScript`)